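; BP_Shelf is a breakable shelf built on a destructible mesh that shows a text message when interacted with.
; When the mesh fractures, it applies a strong impulse along the hit direction, disables the Box collision and sets Broken.
; Interact displays its text through the interactor only while the shelf is unbroken, and PickupActor always returns false.
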(event `self.SM_Shelf_DM.OnComponentFracture`
  (params (HitPoint :type "Vector Structure (by ref)") (HitDirection :type "Vector Structure (by ref)"))
  (`PrimitiveComponent.AddImpulseAtLocation` (`self.SM_Shelf_DM`) (* HitDirection 10000.0) HitPoint "None")
  (`PrimitiveComponent.SetCollisionEnabled` (`self.Box`) "NoCollision")
  (set `self.Broken` true))

(event `self.Interact`
  (params (Interactor :type "Actor Object Reference"))
  (if (not (`self.Broken`))
    (message `Interaction.DisplayInteractionText` Interactor (`self.Text`))))

(fn `PickupActor`
  (params (Actor :type "PickapableActorBase Object Reference"))
  (returns (ReturnValue :type Boolean))
  (return false))

(fn `UserConstructionScript`)