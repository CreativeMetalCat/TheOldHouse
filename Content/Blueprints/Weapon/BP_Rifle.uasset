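; Rifle weapon Blueprint that handles the visual, audio and spawning side of firing and reloading.
; Fire plays the rifle animation, then spawns a bullet at the muzzle socket and an empty shell at the eject socket.
; PlayReloadEffects runs a timeline whose events spawn BP_EmptyShell at the clip-drop socket and play pistol eject and insert sounds.
; Reload itself is empty, and a pistol reload animation is left unconnected.
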(event `self.Fire`
  (params (Location :type "Vector Structure") (Rotation :type "Rotator Structure"))
  (`SkeletalMeshComponent.PlayAnimation` (`self.SkeletalMesh`) "/Game/MilitaryWeapSilver/Weapons/Animations/Fire_Rifle_W.Fire_Rifle_W" false)
  (`|SpawnActorFromClass` "/Game/Blueprints/Weapon/Bullets/BP_Bullet.BP_Bullet_C" (`SceneComponent.GetSocketTransform` (`self.SkeletalMesh`) "MuzzleFlash" "RTS_World") "AlwaysSpawn" "OverrideRootScale" null null)
  (`|SpawnActorFromClass` "/Game/Blueprints/Weapon/Clips/BP_EmptyShell.BP_EmptyShell_C" (`SceneComponent.GetSocketTransform` (`self.SkeletalMesh`) "AmmoEject" "RTS_World") "AdjustIfPossibleButAlwaysSpawn" "OverrideRootScale" null null))

(event `self.Reload`)

(event `self.PlayReloadEffects`
  (`Timeline|ReloadEffects` :!via `PlayFromStart`
    (:`ClipDrop`
      (`|SpawnActorFromClass` "/Game/Blueprints/Weapon/Clips/BP_EmptyShell.BP_EmptyShell_C" (`SceneComponent.GetSocketTransform` (`self.SkeletalMesh`) "ClipDropSocket" "RTS_World") "AdjustIfPossibleButAlwaysSpawn" "OverrideRootScale" null null)
      (`GameplayStatics.PlaySoundAtLocation` "/Game/MilitaryWeapSilver/Sound/Pistol/Cues/Pistol_ReloadEject_Cue.Pistol_ReloadEject_Cue" (`self.K2_GetActorLocation`) (struct) 1.0 1.0 0.0 null null null))
    (:`Sound`
      (`GameplayStatics.PlaySoundAtLocation` "/Game/MilitaryWeapSilver/Sound/Pistol/Cues/Pistol_ReloadInsert_Cue.Pistol_ReloadInsert_Cue" (`self.K2_GetActorLocation`) (struct) 1.0 1.0 0.0 null null null))))

(fn `UserConstructionScript`)