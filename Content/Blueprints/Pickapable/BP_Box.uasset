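; BP_Box is a physics box actor that an interactor can pick up and drop.
; On Interact it hands itself to the interactor through a PickupActor interface message.
; Pickup and drop events toggle actor collision and physics simulation on its mesh, off while held and back on when dropped.
; Its own PickupActor implementation just returns false.
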(event `self.Interact`
  (params (Interactor :type "Actor Object Reference"))
  (message `Interaction.PickupActor` Interactor self))

(event `self.OnDropped`
  (`self.SetActorEnableCollision` true)
  (`PrimitiveComponent.SetSimulatePhysics` (`self.SM_Boxes_04a`) true))

(event `self.OnPickedUp`
  (`self.SetActorEnableCollision` false)
  (`PrimitiveComponent.SetSimulatePhysics` (`self.SM_Boxes_04a`) false))

(fn `PickupActor`
  (params (Actor :type "PickapableActorBase Object Reference"))
  (returns (ReturnValue :type Boolean))
  (return false))

(fn `UserConstructionScript`)